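; Grenade actor that explodes on its first hit, likely an enemy projectile given the damage box it spawns.
; The Hit event plays explosion particles and sound at the impact point, then fires a RadialForce impulse.
; It shakes the player's camera through a cast to mc, spawns EnemyGrenadeExplosionDamageBox to handle damage and destroys itself.
; These last three steps run only if that cast succeeds.
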(event `self.ReceiveHit`
  (params (MyComp :type "PrimitiveComponent Object Reference") (Other :type "Actor Object Reference") (OtherComp :type "PrimitiveComponent Object Reference") (bSelfMoved :type Boolean) (HitLocation :type "Vector Structure") (HitNormal :type "Vector Structure") (NormalImpulse :type "Vector Structure") (Hit :type "HitResult Structure (by ref)"))
  (`GameplayStatics.SpawnEmitterAtLocation` "/Game/SciFiWeapDark/FX/Particles/P_Grenade_Explosion_Light.P_Grenade_Explosion_Light" HitLocation (struct) (0.7 0.7 0.7))
  (`GameplayStatics.SpawnSoundAtLocation` "/Game/SciFiWeapDark/Sound/GrenadeLauncher/Wavs/GrenadeLauncher_Explosion01.GrenadeLauncher_Explosion01" HitLocation (struct) 1.0 1.0 0.0 null null)
  (`|ExecutionSequence`
    (:`then_1`
      (`RadialForceComponent.FireImpulse` (`self.RadialForce`))
      (bind _asthird_person_character (cast `/Game/ThirdPersonBP/Blueprints/mc` (`GameplayStatics.GetPlayerCharacter` 0)))
      (`/Game/ThirdPersonBP/Blueprints/mc.Recoil_Shake` _asthird_person_character 2.0 0.0)
      (`|SpawnActorFromClass` "/Game/Blueprints/EnemyGrenadeExplosionDamageBox.EnemyGrenadeExplosionDamageBox_C" (`KismetMathLibrary.MakeTransform` HitLocation) "Undefined" "OverrideRootScale" null (`self.Instigator`))
      (`self.K2_DestroyActor`))))

(fn `UserConstructionScript`)