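; EnergyShield is an actor that keeps itself attached to the player's shield position.
; Every Tick it casts the first player character to the mc class and moves its root component to the world location and rotation of that character's ShieldLocation component.
; BeginPlay, overlap and construction logic are empty, so it only follows the player by per-frame transform copying.
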(event `self.ReceiveBeginPlay`)

(event `self.ReceiveTick`
  (params (DeltaSeconds :type "Float (single-precision)"))
  (bind _asthird_person_character (cast `/Game/ThirdPersonBP/Blueprints/mc` (`GameplayStatics.GetPlayerCharacter` 0)))
  (`SceneComponent.K2_SetWorldLocationAndRotation` (`self.DefaultSceneRoot`) (.location (`SceneComponent.K2_GetComponentToWorld` (`/Game/ThirdPersonBP/Blueprints/mc.ShieldLocation` _asthird_person_character))) (.rotation (`SceneComponent.K2_GetComponentToWorld` (`/Game/ThirdPersonBP/Blueprints/mc.ShieldLocation` _asthird_person_character))) false false))

(fn `UserConstructionScript`)