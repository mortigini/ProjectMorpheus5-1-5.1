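; Intel pickup that awards a random amount of intel, rolled at BeginPlay between set bounds.
; When the mc character enters its sphere, it removes the Ww component and spawns a particle effect.
; It then eases the Intel component toward the player's WatchSocket, calls AddIntel with the amount and card image, and destroys itself.
; Until pickup, Tick holds Ww at zero world rotation.
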(event `self.ReceiveBeginPlay`
  (set `self.Amount` (`KismetMathLibrary.RandomInteger64InRange` (`self.AmountMin`) (`self.AmountMax`))))

(event `self.Sphere.OnComponentBeginOverlap`
  (params (OverlappedComponent :type "PrimitiveComponent Object Reference") (OtherActor :type "Actor Object Reference") (OtherComp :type "PrimitiveComponent Object Reference") (OtherBodyIndex :type Integer) (bFromSweep :type Boolean) (SweepResult :type "HitResult Structure (by ref)"))
  (cast `/Game/ThirdPersonBP/Blueprints/mc` OtherActor)
  (`ActorComponent.K2_DestroyComponent` (`self.ww`))
  (set `self.Destroyed` true)
  (`GameplayStatics.SpawnEmitterAtLocation` "/Game/SciFiWeapDark/FX/Particles/IntelCollectibleParticle.IntelCollectibleParticle" (`SceneComponent.K2_GetComponentLocation` (`self.Intel`)) (struct) (0.7 0.7 0.7))
  (bind _asthird_person_character (cast `/Game/ThirdPersonBP/Blueprints/mc` (`GameplayStatics.GetPlayerCharacter` 0)))
  (`KismetSystemLibrary.MoveComponentTo` (`self.Intel`) (`SceneComponent.GetSocketLocation` (`Character.Mesh` _asthird_person_character) "WatchSocket") (struct) true true 0.3)
  (bind _asthird_person_character_2 (cast `/Game/ThirdPersonBP/Blueprints/mc` (`GameplayStatics.GetPlayerCharacter` 0)))
  (`/Game/ThirdPersonBP/Blueprints/mc.AddIntel` _asthird_person_character_2 (`self.Amount`) "INTEL" "/Game/UI/card.card" "+")
  (`self.K2_DestroyActor`))

(event `self.ReceiveTick`
  (params (DeltaSeconds :type "Float (single-precision)"))
  (if (not (`self.Destroyed`))
    (`SceneComponent.K2_SetWorldRotation` :`self` (`self.ww`))))

(fn `UserConstructionScript`)