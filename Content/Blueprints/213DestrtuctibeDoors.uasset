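; Destructible door actor with an overhead health bar that explodes and destroys itself when health runs out.
; OpenOneLock removes one health point when the passed value matches the door's index, then refreshes the bar or triggers destruction.
; AnyDamage reveals the bar and runs the same check without subtracting health.
; Once hit, sphere overlap shows the bar again, and the player character leaving hides it.
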(event `self.ReceiveBeginPlay`
  (bind _asover_head_uihealth_bar (cast `/Game/AI/OverHeadUIHealthBar` (`WidgetComponent.GetUserWidgetObject` (`self.HealthBar`))))
  (set `/Game/AI/OverHeadUIHealthBar.Health` (`self.player_health`) _asover_head_uihealth_bar)
  (set `/Game/AI/OverHeadUIHealthBar.PlayerMaxHealth` (`self.player_health_max`) _asover_head_uihealth_bar))

(event `self.ReceiveAnyDamage`
  (params (Damage :type "Float (single-precision)") (DamageType :type "DamageType Object Reference") (InstigatedBy :type "Controller Object Reference") (DamageCauser :type "Actor Object Reference"))
  (set `self.WasHit` true)
  (`|ExecutionSequence`
    (:`then_0`
      (if (<= (`self.player_health`) 0.0) :!label _label
        (`GameplayStatics.SpawnEmitterAtLocation` "/Game/Realistic_Starter_VFX_Pack_Vol2/Particles/Explosion/P_Explosion_Big_B.P_Explosion_Big_B" (`SceneComponent.K2_GetComponentLocation` (`self.Cube`)))
        (`self.K2_DestroyActor`)
        (else
          (bind _asover_head_uihealth_bar (cast `/Game/AI/OverHeadUIHealthBar` (`WidgetComponent.GetUserWidgetObject` (`self.HealthBar`))))
          (set `/Game/AI/OverHeadUIHealthBar.Health` (`self.player_health`) _asover_head_uihealth_bar))))
    (:`then_1`
      (cast `/Game/ThirdPersonBP/Blueprints/mc` (`GameplayStatics.GetPlayerCharacter` 0) :!label _label_2)
      (`SceneComponent.SetVisibility` (`self.HealthBar`) true false))))

(event `ShowHealthBar&CheckIfDestroyed`
  (goto _label))

(event `self.Sphere.OnComponentBeginOverlap`
  (params (OverlappedComponent :type "PrimitiveComponent Object Reference") (OtherActor :type "Actor Object Reference") (OtherComp :type "PrimitiveComponent Object Reference") (OtherBodyIndex :type Integer) (bFromSweep :type Boolean) (SweepResult :type "HitResult Structure (by ref)"))
  (if (`self.WasHit`)
    (goto _label_2)))

(event `self.Sphere.OnComponentEndOverlap`
  (params (OverlappedComponent :type "PrimitiveComponent Object Reference") (OtherActor :type "Actor Object Reference") (OtherComp :type "PrimitiveComponent Object Reference") (OtherBodyIndex :type Integer))
  (cast `/Game/ThirdPersonBP/Blueprints/mc` OtherActor)
  (`SceneComponent.SetVisibility` (`self.HealthBar`) false false))

(fn `OpenOneLock`
  (params (MatchValue :type Integer64))
  (if (== MatchValue (`self.MatchIndexValue`))
    (set `self.WasHit` true)
    (set `self.player_health` (- (`self.player_health`) 1.0))
    (`self.ShowHealthBar&CheckIfDestroyed`)
    (return)))

(fn `UserConstructionScript`)