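; DestructibleCube is a damageable cube actor with an overhead health bar that explodes in a metal destruction effect when its health runs out.
; AnyDamage subtracts from its health, updates the OverHeadUIHealthBar widget, shows the bar and marks the cube as hit.
; Once hit, a Sphere begin overlap shows the bar again, while the mc player character leaving the sphere hides it.
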(event `self.ReceiveBeginPlay`
  (bind _asover_head_uihealth_bar (cast `/Game/AI/OverHeadUIHealthBar` (`WidgetComponent.GetUserWidgetObject` (`self.HealthBar`))))
  (set `/Game/AI/OverHeadUIHealthBar.Health` (`self.player_health`) _asover_head_uihealth_bar)
  (set `/Game/AI/OverHeadUIHealthBar.PlayerMaxHealth` (`self.player_health_max`) _asover_head_uihealth_bar))

(event `self.ReceiveAnyDamage`
  (params (Damage :type "Float (single-precision)") (DamageType :type "DamageType Object Reference") (InstigatedBy :type "Controller Object Reference") (DamageCauser :type "Actor Object Reference"))
  (set `self.WasHit` true)
  (`|ExecutionSequence`
    (:`then_0`
      (set `self.player_health` (- (`self.player_health`) Damage))
      (if (<= (`self.player_health`) 0.0)
        (`GameplayStatics.SpawnEmitterAtLocation` "/Game/Realistic_Starter_VFX_Pack_Vol2/Particles/Destruction/P_Destruction_Metal.P_Destruction_Metal" (`SceneComponent.K2_GetComponentLocation` (`self.Cube`)) (struct) (3.0 3.0 3.0))
        (`self.K2_DestroyActor`)
        (else
          (bind _asover_head_uihealth_bar (cast `/Game/AI/OverHeadUIHealthBar` (`WidgetComponent.GetUserWidgetObject` (`self.HealthBar`))))
          (set `/Game/AI/OverHeadUIHealthBar.Health` (`self.player_health`) _asover_head_uihealth_bar))))
    (:`then_1`
      (cast `/Game/ThirdPersonBP/Blueprints/mc` (`GameplayStatics.GetPlayerCharacter` 0) :!label _label)
      (`SceneComponent.SetVisibility` (`self.HealthBar`) true false))))

(event `self.Sphere.OnComponentBeginOverlap`
  (params (OverlappedComponent :type "PrimitiveComponent Object Reference") (OtherActor :type "Actor Object Reference") (OtherComp :type "PrimitiveComponent Object Reference") (OtherBodyIndex :type Integer) (bFromSweep :type Boolean) (SweepResult :type "HitResult Structure (by ref)"))
  (if (`self.WasHit`)
    (goto _label)))

(event `self.Sphere.OnComponentEndOverlap`
  (params (OverlappedComponent :type "PrimitiveComponent Object Reference") (OtherActor :type "Actor Object Reference") (OtherComp :type "PrimitiveComponent Object Reference") (OtherBodyIndex :type Integer))
  (cast `/Game/ThirdPersonBP/Blueprints/mc` OtherActor)
  (`SceneComponent.SetVisibility` (`self.HealthBar`) false false))

(fn `UserConstructionScript`)